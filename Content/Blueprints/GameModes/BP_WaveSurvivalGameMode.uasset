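; Game mode Blueprint for wave survival that shows on-screen wave announcements as the match state changes.
; It binds to the state-changed delegate on BeginPlay and routes each state to its own handler.
; Handlers spawn countdown or plain text widgets for incoming, active, final and completed waves.
; All-waves-cleared and player-death handlers only print placeholder strings; spawning logic is not in this graph.
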(event `self.ReceiveBeginPlay`
  (add `self.OnWaveSurvivalGameModeStateChanged` (`|CreateDelegate` :!event `OnWaveSurvivalGameModeStateChanged_Event`)))

(event `OnWaveSurvivalGameModeStateChanged_Event` :!signature `self.OnWaveSurvivalGameModeStateChanged`
  (params (NewState :type "EAGWaveSurvivalGameModeState Enum" :default "WaitToSpawnNewWave"))
  (switch `EAGWaveSurvivalGameModeState` NewState
    (:`WaitToSpawnNewWave`
      (`self.OnWaitToSpawnNewWave`))
    (:`SpawningNewWave`
      (`self.OnSpawningNewWave`))
    (:`WaveCompleted`
      (`self.OnWaveCompleted`))
    (:`AllWavesCleared`
      (`self.OnAllWavesCleared`))
    (:`PlayerDied`
      (`self.OnPlayerDied`))))

(event `OnWaitToSpawnNewWave`
  (`self.CreateWaveWidgetWithCountDown` (`|FormatText` "Wave {CurrentWaveCount} is comming in" (`self.CurrentWaveCount`)) (`self.SpawnNewWaveWaitTime`)))

(event `OnSpawningNewWave`
  (`self.CreateWaveWidgetNoCountDown` (`|FormatText` "Wave {CurrentWaveCount}" (`self.CurrentWaveCount`)))
  (if (== (`self.CurrentWaveCount`) (`self.TotalWavesToSpawn`))
    (`KismetSystemLibrary.Delay` 2.0)
    (`self.CreateWaveWidgetNoCountDown` "Last Wave")))

(event `OnWaveCompleted`
  (`self.CreateWaveWidgetWithCountDown` (`|FormatText` "Wave {CurrentWaveCount} completed" (`self.CurrentWaveCount`)) (`self.WaveCompletedWaitTime`)))

(event `OnAllWavesCleared`
  (`KismetSystemLibrary.PrintString` "Period"))

(event `OnPlayerDied`
  (`KismetSystemLibrary.PrintString` "EW"))

(fn `CreateWaveWidgetNoCountDown`
  (params (InDisplayTextContent :type Text))
  (bind _returnvalue (`|CreateWidget` "/Game/Blueprints/UI/Widgets/GameModeWidgets/WBP_WaveTextNoCooldown.WBP_WaveTextNoCooldown_C" (`GameplayStatics.GetPlayerController` 0)))
  (`UserWidget.AddToViewport` _returnvalue 0)
  (`TextBlock.SetText` (`/Game/Blueprints/UI/Widgets/GameModeWidgets/WBP_WaveTextNoCooldown.WaveText_TextBlock` _returnvalue) (`local.InDisplayTextContent`)))

(fn `CreateWaveWidgetWithCountDown`
  (params (InTextContentToDisplay :type Text) (InTotalCountDownTime :type "Float (double-precision)"))
  (bind _returnvalue (`|CreateWidget` "/Game/Blueprints/UI/Widgets/GameModeWidgets/WBP_WaveTextWithCooldown.WBP_WaveTextWithCooldown_C" (`GameplayStatics.GetPlayerController` 0)))
  (`UserWidget.AddToViewport` _returnvalue 0)
  (`TextBlock.SetText` (`/Game/Blueprints/UI/Widgets/GameModeWidgets/WBP_WaveTextWithCooldown.WaveText_TextBlock` _returnvalue) (`local.InTextContentToDisplay`))
  (`/Game/Blueprints/UI/Widgets/GameModeWidgets/WBP_WaveTextWithCooldown.StartCountDown` _returnvalue (`local.InTotalCountDownTime`)))

(fn `UserConstructionScript`)