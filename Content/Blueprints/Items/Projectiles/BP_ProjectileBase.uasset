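; Base projectile Blueprint that handles the sound and visual effects for spawning, flight and impact.
; On BeginPlay it plays a spawn sound, attaches a flying sound to the root and spawns a forward-facing muzzle system, each when valid.
; OnSpawnProjectileHitFX plays the impact sound and spawns the impact effect at the supplied hit location.
; The graph contains no movement, collision or damage logic.
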(event `self.ReceiveBeginPlay`
  (`|ExecutionSequence`
    (:`then_0`
      (bind _projectilespawnsound (`self.ProjectileSpawnSound`)
        (:`then`
          (`GameplayStatics.PlaySoundAtLocation` _projectilespawnsound (`self.K2_GetActorLocation`) (struct) 0.3 1.0 0.0 null null null null))
        (:`else`)))
    (:`then_1`
      (bind _projectileflyingsound (`self.ProjectileFlyingSound`)
        (:`then`
          (`GameplayStatics.SpawnSoundAttached` _projectileflyingsound (`self.RootComponent`) "None" (0.0 0.0 0.0) (struct) "KeepRelativeOffset" true 0.3 1.0 0.0 null null))
        (:`else`)))
    (:`then_2`
      (bind _projectilemuzzlefx (`self.ProjectileMuzzleFX`)
        (:`then`
          (`NiagaraFunctionLibrary.SpawnSystemAtLocation` _projectilemuzzlefx (`self.K2_GetActorLocation`) (`KismetMathLibrary.Conv_VectorToRotator` (`self.GetActorForwardVector`))))
        (:`else`)))))

(event `self.BP_OnSpawnProjectileHitFX`
  (params (HitLocation :type "Vector Structure (by ref)"))
  (`|ExecutionSequence`
    (:`then_0`
      (`GameplayStatics.PlaySoundAtLocation` (`self.ProjectileImpactSound`) HitLocation (struct) (`self.ProjectileImpactSoundVolume`) 1.0 0.0 null null null null))
    (:`then_1`
      (bind _projectileimpactfx (`self.ProjectileImpactFX`)
        (:`then`
          (`NiagaraFunctionLibrary.SpawnSystemAtLocation` _projectileimpactfx HitLocation))
        (:`else`)))))

(fn `UserConstructionScript`)