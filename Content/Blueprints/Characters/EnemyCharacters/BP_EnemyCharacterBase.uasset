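; Base Blueprint for enemy characters that handles the dissolve effect when an enemy dies.
; OnEnemyDied disables capsule collision, pauses animations and async-loads the given Niagara system, which spawns on the mesh tinted with the material's DissolveEdgeColor.
; A timeline scaled to TotalDissolveTime drives DissolveAmount on the body and equipped weapon materials, then destroys both weapon and character.
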(event `self.ReceiveBeginPlay`)

(event `/Game/Blueprints/Characters/EnemyCharacters/BPI_Enemy_Death.OnEnemyDied`
  (params (DissolveNiagaraSystem :type "NiagaraSystem Soft Object Reference"))
  (bind _returnvalue (`PawnCombatComponent.GetCharacterCurrentEquippedWeapon` (`self.EnemyCombatComponent`)))
  (`|ExecutionSequence`
    (:`then_0`
      ;[1 1 1] Disable collision and pause animations
      (set `SkeletalMeshComponent.bPauseAnims` true (`self.Mesh`))
      (`PrimitiveComponent.SetCollisionEnabled` (`self.CapsuleComponent`) "NoCollision"))
    (:`then_1`
      ;[1 1 1] Dissolve enemy and weapon
      (bind _object (`|LoadAsset` DissolveNiagaraSystem)
        (:`Completed`
          (bind _asniagara_system (cast `NiagaraSystem` _object)
            (:`then`
              (`self.SetDeathNiagaraSystem` _asniagara_system))
            (:`CastFailed`
              _))
          (`TimelineComponent.SetPlayRate` (`self.DissolveTimeline`) (/ 1.0 (`self.TotalDissolveTime`)))
          (bind (_direction _normalizedfloattrack) (`Timeline|DissolveTimeline` :!via `PlayFromStart`)
            (:`Update`
              (`self.SetDissolveMaterial` _normalizedfloattrack))
            (:`Finished`
              (`/Engine/EditorBlueprintResources/StandardMacros.IsValid` _returnvalue
                (:`Is Valid`
                  (`self.K2_DestroyActor` _returnvalue))
                (:`Is Not Valid`
                  _))
              (`self.K2_DestroyActor`))))))))

(fn `SetDeathNiagaraSystem`
  (params (DeathNiagaraSystem :type "NiagaraSystem Object Reference"))
  (bind _mesh (`self.Mesh`))
  (bind _returnvalue (`NiagaraFunctionLibrary.SpawnSystemAttached` DeathNiagaraSystem (`self.Mesh`) "None" (0.0 0.0 0.0) (struct) "KeepRelativeOffset" true))
  (bind _returnvalue_2 (`PrimitiveComponent.CreateDynamicMaterialInstance` _mesh 0 (`PrimitiveComponent.GetMaterial` _mesh 0) "None"))
  (bind _returnvalue_3 (`MaterialInstanceDynamic.K2_GetVectorParameterValue` _returnvalue_2 "DissolveEdgeColor"))
  (`NiagaraComponent.SetNiagaraVariableLinearColor` _returnvalue "DissolveParticleColor" _returnvalue_3))

(fn `SetDissolveMaterial`
  (params (DissolveValue :type "Float (single-precision)"))
  (bind _returnvalue (`PawnCombatComponent.GetCharacterCurrentEquippedWeapon` (`self.EnemyCombatComponent`)))
  (`MeshComponent.SetScalarParameterValueOnMaterials` (`self.Mesh`) "DissolveAmount" DissolveValue)
  (`/Engine/EditorBlueprintResources/StandardMacros.IsValid` _returnvalue
    (:`Is Valid`
      (`MeshComponent.SetScalarParameterValueOnMaterials` (`AGWeaponBase.WeaponMesh` _returnvalue) "DissolveAmount" (`local.DissolveValue`)))))

(fn `UserConstructionScript`)