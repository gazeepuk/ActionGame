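; GA_LightAttack_Pistol is a hero light pistol attack ability that picks a shoot target from the camera view on activation.
; When target-locked, it line traces along camera forward up to ShootDistance.
; Otherwise, TryFaceToTarget runs a debug-drawn sphere trace and sets the "TargetActor" motion warping location to the impact point for aim assist.
; Either hit actor is stored in ShootTarget, but the following validity check leads to no further logic.
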(event `self.K2_ActivateAbility`
  (bind _returnvalue (`GameplayStatics.GetPlayerCameraManager` 0))
  (bind _returnvalue_2 (`Actor.K2_GetActorLocation` _returnvalue))
  (`parent.K2_ActivateAbility`)
  (`AGFunctionLibrary.BP_DoesActorHaveTag` (`self.GetAvatarActorFromActorInfo`) (struct :`TagName` "Player.Status.TargetLock")
    (:`Yes`
      ;[1 1 1] Trace locked target
      (bind _outhit (`KismetSystemLibrary.LineTraceSingleForObjects` _returnvalue_2 (+ _returnvalue_2 (* (`Actor.GetActorForwardVector` _returnvalue) (`self.ShootDistance`))) (`self.Object Types`)))
      (set `self.ShootTarget` (`.HitActor` (`GameplayStatics.BreakHitResult` _outhit))))
    (:`No`
      ;[1 1 1] Trace and adjust rotation to target
      (bind _outhitresult (`self.TryFaceToTarget`))
      (set `self.ShootTarget` (`.HitActor` (`GameplayStatics.BreakHitResult` _outhitresult)))))
  (`self.ShootTarget`
    (:`then`)
    (:`else`)))

(fn `TryFaceToTarget`
  (returns (OutHitResult :type "HitResult Structure"))
  (bind _returnvalue (`GameplayStatics.GetPlayerCameraManager` 0))
  (bind _returnvalue_2 (`Actor.K2_GetActorLocation` _returnvalue))
  (bind (_outhit _returnvalue_3) (`KismetSystemLibrary.SphereTraceSingleForObjects` :`Start` _returnvalue_2 :`End` (+ _returnvalue_2 (* (`Actor.GetActorForwardVector` _returnvalue) (`self.ShootDistance`))) :`Radius` 200.0 :`ObjectTypes` (`self.Object Types`) :`DrawDebugType` "ForDuration"))
  (if _returnvalue_3
    (`MotionWarpingComponent.AddOrUpdateWarpTargetFromLocation` (`AGBaseCharacter.MotionWarping` (`self.GetHeroCharacterFromActorInfo`)) "TargetActor" (`.ImpactPoint` (`GameplayStatics.BreakHitResult` _outhit)))
    (return _outhit)))