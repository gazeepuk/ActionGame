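; Hero pistol light attack ability that spends ammo through TryShoot and hits a target found by camera-forward sphere traces, ending if the shot fails.
; With target lock it uses a narrow trace; otherwise TryFaceToTarget uses a wider one and sets a motion warp target at the impact point.
; Hit actors go to the hero combat component, whose overlapped actors reset on end.
; HandleApplyDamage adds a special pistol effect while Rage is active.
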(event `self.K2_ActivateAbility`
  (bind _returnvalue (`GameplayStatics.GetPlayerCameraManager` 0))
  (bind _returnvalue_2 (`Actor.K2_GetActorLocation` _returnvalue))
  (`parent.K2_ActivateAbility`)
  (bind _asaghero_ammo_weapon (cast `AGHeroAmmoWeapon` (`PawnCombatComponent.GetCharacterCurrentEquippedWeapon` (`self.GetHeroCombatComponentFromActorInfo`)))
    (:`then`
      (bind _returnvalue_3 (`AGHeroAmmoWeapon.TryShoot` _asaghero_ammo_weapon (`self.ShotAmmoCost`)))
      (if _returnvalue_3
        (`AGFunctionLibrary.BP_DoesActorHaveTag` (`self.GetAvatarActorFromActorInfo`) (struct :`TagName` "Player.Status.TargetLock")
          (:`Yes`
            ;[1 1 1] Trace locked target
            (bind _outhit (`KismetSystemLibrary.SphereTraceSingleForObjects` _returnvalue_2 (+ _returnvalue_2 (* (`Actor.GetActorForwardVector` _returnvalue) (`self.ShootDistance`))) 50.0 (`self.Object Types`)))
            (set `self.ShootTarget` (`.HitActor` (`GameplayStatics.BreakHitResult` _outhit))))
          (:`No`
            ;[1 1 1] Trace and adjust rotation to target
            (bind _outhitresult (`self.TryFaceToTarget`))
            (set `self.ShootTarget` (`.HitActor` (`GameplayStatics.BreakHitResult` _outhitresult)))))
        (bind _shoottarget (`self.ShootTarget`)
          (:`then`
            (`PawnCombatComponent.OnHitTargetActor` (`self.GetHeroCombatComponentFromActorInfo`) _shoottarget))
          (:`else`))
        (else
          (`self.K2_EndAbility` :!label _label))))
    (:`CastFailed`
      (goto _label))))

(event `self.K2_OnEndAbility`
  (params (bWasCancelled :type Boolean))
  (`parent.K2_OnEndAbility` bWasCancelled)
  (`PawnCombatComponent.ResetOverlappedActors` (`self.GetHeroCombatComponentFromActorInfo`)))

(fn `HandleApplyDamage`
  (params (GameplayEventData :type "GameplayEventData Structure (by ref)"))
  (`parent.HandleApplyDamage` GameplayEventData)
  ;[1 1 1] Apply GameplayEffect to Target if Rage is Active
  (`AGFunctionLibrary.BP_DoesActorHaveTag` (`self.GetAvatarActorFromActorInfo`) (struct :`TagName` "Player.Status.Rage.Active")
    (:`Yes`
      (`self.BP_ApplyEffectSpecHandleToTarget` (`.Target` (break `GameplayEventData` GameplayEventData)) (`self.MakeOutgoingGameplayEffectSpec` "/Game/Blueprints/AbilitySystem/GameplayEffects/Hero/SpecialWeaopon/Pistol/Light/GE_Hero_SpecialWeapon_Light_Pistol.GE_Hero_SpecialWeapon_Light_Pistol_C" (`KismetMathLibrary.Conv_IntToDouble` (`self.GetAbilityLevel`)))
        (:`Successful`
          _)
        (:`Failed`
          _))
      (return))))

(fn `TryFaceToTarget`
  (returns (OutHitResult :type "HitResult Structure"))
  (bind _returnvalue (`GameplayStatics.GetPlayerCameraManager` 0))
  (bind _returnvalue_2 (`Actor.K2_GetActorLocation` _returnvalue))
  (bind _motionwarping (`AGBaseCharacter.MotionWarping` (`self.GetHeroCharacterFromActorInfo`)))
  (bind (_outhit _returnvalue_3) (`KismetSystemLibrary.SphereTraceSingleForObjects` _returnvalue_2 (+ _returnvalue_2 (* (`Actor.GetActorForwardVector` _returnvalue) (`self.ShootDistance`))) 200.0 (`self.Object Types`)))
  (if _returnvalue_3
    (`MotionWarpingComponent.AddOrUpdateWarpTargetFromLocation` _motionwarping "TargetActor" (`.ImpactPoint` (`GameplayStatics.BreakHitResult` _outhit)))
    (return _outhit)
    (else
      (`MotionWarpingComponent.RemoveWarpTarget` _motionwarping "TargetActor")
      (return))))